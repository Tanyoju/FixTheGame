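; BP_Wendigo is an enemy character that hunts the player and is banished by the player's lantern.
; It reissues an AI MoveTo to the player's location every Tick and, if the lantern is on, notifies the player and destroys itself regardless of distance.
; A punch-range overlap triggers a montage attack that, after a short delay and range recheck, damages the player and launches them along the Wendigo's forward vector.
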(event `self.ReceiveBeginPlay`
  (`self.Chase`))

(event `self.ReceiveTick`
  (params (DeltaSeconds :type "Float (single-precision)"))
  (`self.Chase`))

(event `Chase`
  (bind _asbp_custom_tps (cast `/Game/Blueprints/BP_CustomTPS` (`GameplayStatics.GetPlayerCharacter` 0)))
  (`|AIMoveTo` self (`self.K2_GetActorLocation` _asbp_custom_tps) null
    (:`then`
      (if (`/Game/Blueprints/BP_CustomTPS.LanternOn` _asbp_custom_tps)
        (`/Game/Blueprints/BP_CustomTPS.DestroyWendigo` _asbp_custom_tps)
        (`self.K2_DestroyActor`)))))

(event `self.PunchRange.OnComponentBeginOverlap`
  (params (OverlappedComponent :type "PrimitiveComponent Object Reference") (OtherActor :type "Actor Object Reference") (OtherComp :type "PrimitiveComponent Object Reference") (OtherBodyIndex :type Integer) (bFromSweep :type Boolean) (SweepResult :type "HitResult Structure (by ref)"))
  (cast `/Game/Blueprints/BP_CustomTPS` OtherActor)
  (set `self.CanAttackPlayer` true)
  (`self.Attack`))

(event `self.PunchRange.OnComponentEndOverlap`
  (params (OverlappedComponent :type "PrimitiveComponent Object Reference") (OtherActor :type "Actor Object Reference") (OtherComp :type "PrimitiveComponent Object Reference") (OtherBodyIndex :type Integer))
  (cast `/Game/Blueprints/BP_CustomTPS` OtherActor)
  (set `self.CanAttackPlayer` false)
  (`self.Chase`))

(event `Attack`
  (if (`self.CanAttackPlayer`)
    (`self.PlayAnimMontage` "/Game/Animation/Mutant_Punch_Montage.Mutant_Punch_Montage" 0.6)
    (`KismetSystemLibrary.Delay` 0.3)
    (if (`self.CanAttackPlayer`)
      (bind _asbp_custom_tps (cast `/Game/Blueprints/BP_CustomTPS` (stale `self.PunchRange.OnComponentBeginOverlap` OtherActor)))
      (`/Game/Blueprints/BP_CustomTPS.Damage` _asbp_custom_tps)
      (`self.LaunchCharacter` _asbp_custom_tps (* (`KismetMathLibrary.GetForwardVector` (`self.K2_GetActorRotation`)) 6000.0) true true))))

(fn `UserConstructionScript`)